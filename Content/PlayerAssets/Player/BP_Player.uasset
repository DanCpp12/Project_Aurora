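; Player character Blueprint handling sword attacks, interaction, damage and death.
; Light attack plays a slash montage, while TriggerSword and StopTriggerSword control a looping timer that line-traces between blade sockets and applies damage on every tick.
; Incoming damage is DoOnce-gated through the hit reaction, and death disables control, plays a montage and destroys the actor.
; Interact messages the stored area actor, and debug keys exercise Burn tags on a gameplay tag component.
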(event Custom|TriggerSword
  ;[0 0.0615 1] Attack & DealDamage
  (bind _returnvalue (Utilities|Time|SetTimerbyEvent (delegate Custom|SwordLineTrace) 0.001 true))
  (Variables|Default|SetTriggerSwordEvent _returnvalue))

(event Custom|SwordLineTrace
  (bind _swordmesh (Variables|Default|GetswordMesh))
  ;[0 0.0615 1] Attack & DealDamage
  (bind _outhit (Collision|LineTraceByChannel (Transformation|GetSocketLocation _swordmesh "start") (Transformation|GetSocketLocation _swordmesh "end") "TraceTypeQuery2" false 0 "ForDuration"))
  (Game|Damage|ApplyDamage (.HitActor (Collision|BreakHitResult _outhit)) (Variables|Default|GetDamage) 0 0 "/Script/Engine.DamageType"))

(event Custom|StopTriggerSword
  ;[0 0.0615 1] Attack & DealDamage
  (Utilities|Time|ClearandInvalidateTimerbyHandle (Variables|Default|GetTriggerSwordEvent)))

(event Custom|BurnChanged
  (params (GameplayTagContext :type F%20Gameplay%20Context%20Structure))
  (Development|PrintString "BurnTagChanged" true true "(R=0.000000,G=0.660000,B=1.000000,A=1.000000)" 2.0 "1"))

(event Input|EnhancedActionEvents|EnhancedInputActionIA_Interact
  (params (ActionValue :type Boolean) (ElapsedSeconds :type Float%20%28double-precision%29) (TriggeredSeconds :type Float%20%28double-precision%29) (InputAction :type Input%20Action%20Object%20Reference :default "/Game/Input/InputActions/IA_Interact.IA_Interact"))
  (Class|BPIInteract|OnInteract(Message) (Variables|Default|GetActor%20to%20Interact%20With)))

(event Input|EnhancedActionEvents|EnhancedInputActionIA_LightAttack
  (params (ActionValue :type Boolean) (ElapsedSeconds :type Float%20%28double-precision%29) (TriggeredSeconds :type Float%20%28double-precision%29) (InputAction :type Input%20Action%20Object%20Reference :default "/Game/Input/InputActions/IA_LightAttack.IA_LightAttack"))
  ;[0 0.0615 1] Attack & DealDamage
  (Utilities|FlowControl|DoOnce false :!label _label
    (:Completed
      (bind _returnvalue (Animation|PlayAnimMontage "/Game/PlayerAssets/Player/Animations/SwordSlash_Montage.SwordSlash_Montage" 1.0 "None"))
      (Utilities|FlowControl|Delay _returnvalue)
      (goto _label Reset))))

(event Game|Damage|EventAnyDamage
  (params (Damage :type Float%20%28single-precision%29) (DamageType :type Damage%20Type%20Object%20Reference) (InstigatedBy :type Controller%20Object%20Reference) (DamageCauser :type Actor%20Object%20Reference))
  ;[1 0 0.04338] Take Damage
  (Utilities|FlowControl|DoOnce false :!label _label
    (:Completed
      (bind _output_get (Variables|Default|SetHealth (- (Variables|Default|GetHealth) Damage)))
      (if (<= _output_get 0.0)
        (Input|SetInputModeUIOnly (Game|GetPlayerController 0) 0 "DoNotLock" false)
        (Pawn|Components|CharacterMovement|DisableMovement (Variables|Character|GetCharacterMovement))
        (bind _returnvalue (Animation|PlayAnimMontage "/Game/PlayerAssets/Player/Animations/Death_Montage.Death_Montage" 1.0 "None"))
        (Utilities|FlowControl|Delay _returnvalue)
        (Actor|DestroyActor)
        (else
          (bind _returnvalue_2 (Animation|PlayAnimMontage "/Game/PlayerAssets/Player/Animations/HitReact_Montage.HitReact_Montage" 1.0 "None"))
          (Utilities|FlowControl|Delay _returnvalue_2)
          (goto _label Reset))))))

(event Collision|EventActorBeginOverlap
  (params (OtherActor :type Actor%20Object%20Reference)))

(event EventTick
  (params (DeltaSeconds :type Float%20%28single-precision%29)))

(event EventInteractAreaExited
  (params (ActorToInteractWith :type Actor%20Object%20Reference))
  (Variables|Default|SetActor%20to%20Interact%20With ActorToInteractWith))

(event EventInteractAreaEntered
  (params (ActorToInteractWith :type Actor%20Object%20Reference))
  (Variables|Default|SetActor%20to%20Interact%20With ActorToInteractWith))

(event Input|KeyboardEvents|DebugKey1
  (params (Key :type Key%20Structure :default "None") (ActionValue :type Input%20Action%20Value%20Structure))
  (bind _bpac_gameplaytags (Variables|Default|GetBPAC_GameplayTags))
  (:Pressed
    (Default|AddTag _bpac_gameplaytags "(TagName=\"Effect.Burn\")")
    (Default|DebugPrintStackAmount _bpac_gameplaytags "(TagName=\"Effect.Burn\")")))

(event Input|KeyboardEvents|DebugKey3
  (params (Key :type Key%20Structure :default "None") (ActionValue :type Input%20Action%20Value%20Structure))
  (:Pressed
    (Default|AddTagListener (Variables|Default|GetBPAC_GameplayTags) "(TagName=\"Effect.Burn\")" (delegate Custom|BurnChanged))))

(event Input|KeyboardEvents|DebugKey2
  (params (Key :type Key%20Structure :default "None") (ActionValue :type Input%20Action%20Value%20Structure))
  (bind _bpac_gameplaytags (Variables|Default|GetBPAC_GameplayTags))
  (:Pressed
    (Default|RemoveTag _bpac_gameplaytags "(TagName=\"Effect.Burn\")")
    (Default|DebugPrintStackAmount _bpac_gameplaytags "(TagName=\"Effect.Burn\")")))

(fn ConstructionScript)